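; BP_Timer is a countdown timer Blueprint that holds Minutes and Seconds counters.
; Tick feeds a one-second Delay, pacing logic meant to decrement Seconds and roll over to 59 as Minutes drops.
; Both branch conditions are constant true and the zero comparisons for Minutes and Seconds are unconnected, so neither counter changes as wired.
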(event `self.ReceiveTick`
  (params (DeltaSeconds :type "Float (single-precision)"))
  (`KismetSystemLibrary.Delay` 1.0)
  (if true
    (if (not true)
      (`/Engine/EditorBlueprintResources/StandardMacros.DecrementFloat` (`self.Minutes`)
        (:`  `
          (set `self.Seconds` 59.0))))
    (else
      (`/Engine/EditorBlueprintResources/StandardMacros.DecrementFloat` (`self.Seconds`)))))

(fn `UserConstructionScript`)